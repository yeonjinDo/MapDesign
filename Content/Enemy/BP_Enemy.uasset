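; Enemy character for melee combat that takes hits from an attacker, reacts with montages, knockback and camera shake, and dies.
; Damage events store the hit data and set the StateComponent to Hitted, whose change callback subtracts HP and branches on death or skill hits.
; Skill hits use hardcoded hit data and down the enemy, triggering a paired stab finisher at low HP.
; Tick updates HP text, attack permission and a height cap; a sphere tracks nearby targets for facing.
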(event `InputAxis|MoveForward`
  (params (AxisValue :type "Float (single-precision)")))

(event `InputAxis|MoveRight`
  (params (AxisValue :type "Float (single-precision)")))

(event `InputAxis|HorizontalLook`
  (params (AxisValue :type "Float (single-precision)")))

(event `InputAxis|VerticalLook`
  (params (AxisValue :type "Float (single-precision)")))

(event `self.ReceiveBeginPlay`
  (for (_array_element _array_index) (`MeshComponent.GetMaterials` (`self.Mesh`))
    (bind _returnvalue (`KismetMaterialLibrary.CreateDynamicMaterialInstance` _array_element))
    (`KismetArrayLibrary.Array_Add` (`self.Materials`) _returnvalue)
    (`PrimitiveComponent.SetMaterial` (`self.Mesh`) _array_index _returnvalue)
    (`/Game/Components/MovingComponent.OffControlRotation` (`self.MovingComponent`))
    (bind _output_get (set `/Game/Components/HpComponent.MaxHp` (`self.MaxHp`) (`self.HpComponent`)))
    (set `self.Hp` _output_get)
    (add `/Game/Components/StateComponent.OnStateTypeChanged` (`self.StateComponent`) (delegate `OnStateTypeChanged`))))

(event `OnStateTypeChanged`
  (params (InPrevType :type "/Game/Components/EStateType Enum" :default "NewEnumerator0") (InNewType :type "/Game/Components/EStateType Enum" :default "NewEnumerator0"))
  (switch `/Game/Components/EStateType` InNewType
    (:`NewEnumerator5`
      (`self.Hitted`))))

(event `self.Sphere.OnComponentBeginOverlap`
  (params (OverlappedComponent :type "PrimitiveComponent Object Reference") (OtherActor :type "Actor Object Reference") (OtherComp :type "PrimitiveComponent Object Reference") (OtherBodyIndex :type Integer) (bFromSweep :type Boolean) (SweepResult :type "HitResult Structure (by ref)"))
  (if (`KismetStringLibrary.NotEqual_StrStr` (`KismetSystemLibrary.GetClassDisplayName` (`GameplayStatics.GetObjectClass` OtherActor)) (`KismetSystemLibrary.GetClassDisplayName` (`GameplayStatics.GetObjectClass` self)))
    (set `self.NotMyTeam` true)
    (`KismetArrayLibrary.Array_AddUnique` (`self.OtherEnemy`) OtherActor)))

(event `self.Sphere.OnComponentEndOverlap`
  (params (OverlappedComponent :type "PrimitiveComponent Object Reference") (OtherActor :type "Actor Object Reference") (OtherComp :type "PrimitiveComponent Object Reference") (OtherBodyIndex :type Integer))
  (bind _otherenemy (`self.OtherEnemy`))
  (`KismetArrayLibrary.Array_Remove` _otherenemy (`KismetArrayLibrary.Array_Find` _otherenemy OtherActor)))

(event `self.OnLanded`
  (params (Hit :type "HitResult Structure (by ref)"))
  (if (<= 5.0 (`CharacterMovementComponent.GravityScale` (`self.CharacterMovement`)))
    (set `CharacterMovementComponent.GravityScale` 1.0 (`self.CharacterMovement`))
    (`self.PlayAnimMontage` "/Game/Character/Animations/Common/Jump_Landing_Seq_Montage.Jump_Landing_Seq_Montage")))

(event `LookAt`
  (bind _output (`|GetArrayItem` (`self.OtherEnemy`) (`self.EnemyIndex`)))
  (bind (_returnvalue_roll _returnvalue_pitch _returnvalue_yaw) (`KismetMathLibrary.BreakRotator` (`KismetMathLibrary.FindLookAtRotation` (`self.K2_GetActorLocation`) (`self.K2_GetActorLocation` (`self.Attacker`)))))
  (bind (_returnvalue_roll_2 _returnvalue_pitch_2 _returnvalue_yaw_2) (`KismetMathLibrary.BreakRotator` (`KismetMathLibrary.FindLookAtRotation` (`self.K2_GetActorLocation`) (`self.K2_GetActorLocation` _output))))
  (if (`self.temp`)
    _
    (elif (`KismetSystemLibrary.IsValid` _output)
      (`self.K2_SetActorRotation` (`KismetMathLibrary.MakeRotator` 0.0 0.0 _returnvalue_yaw_2))
      (else
        (`self.K2_SetActorRotation` (`KismetMathLibrary.MakeRotator` 0.0 0.0 _returnvalue_yaw))))))

(event `self.ReceiveTick`
  (params (DeltaSeconds :type "Float (single-precision)"))
  (bind _attacker (`self.Attacker`))
  (if (`KismetSystemLibrary.IsValid` _attacker)
    (if (`/Game/Components/StateComponent.IsSkillMode` (`self.GetComponentByClass` _attacker "/Game/Components/StateComponent.StateComponent_C"))
      (set `self.CanAttack` false :!label _label)
      (else
        (set `self.CanAttack` true)))
    (else
      (goto _label)))
  (`TextRenderComponent.K2_SetText` (`self.HPText`) (`KismetTextLibrary.Conv_DoubleToText` (`self.Hp`) "HalfToEven"))
  (if (`self.ParryingSuccess`)
    (`ActorComponent.Activate` (`self.ParticleSystem`) false))
  (`self.LimitHeight`)
  (if (`KismetArrayLibrary.Array_IsValidIndex` (`self.OtherEnemy`) (`self.EnemyIndex`))
    (if (`self.NotMyTeam`)
      (if (and (> (`KismetArrayLibrary.Array_Length` (`self.OtherEnemy`)) 0) (`KismetArrayLibrary.Array_IsValidIndex` (`self.OtherEnemy`) (`self.EnemyIndex`)))
        (`/Engine/EditorBlueprintResources/StandardMacros.IsValid` (`|GetArrayItem` (`self.OtherEnemy`) (`self.EnemyIndex`))
          (:`Is Valid`
            (if (< 0.0 (`self.Hp`))
              _)))))))

(event `Rise`
  (`self.PlayAnimMontage` "/Game/Montages/Damaged/Enemy_EndFaint_Rise_Montage.Enemy_EndFaint_Rise_Montage"))

(event `Faint`
  (`self.Rise`)
  (`/Engine/EditorBlueprintResources/StandardMacros.IsValid` (`self.Attacker`)))

(event `End_Dead`
  (bind _weapon (`/Game/Components/WeaponComponent.GetCurrentWeapon` (`self.WeaponComponent`)))
  (`/Engine/EditorBlueprintResources/StandardMacros.IsValid` _weapon
    (:`Is Valid`
      (`self.K2_DestroyActor` _weapon)
      (`self.K2_DestroyActor`))))

(event `/Game/IDamage.Damaged`
  (params (Attacker :type "Character Object Reference") (Causer :type "Actor Object Reference") (HitData :type "/Game/Weapons/FHitData Structure"))
  (bind _output_get (set `self.Attacker` Attacker))
  (set `self.Causer` Causer)
  (if (not (== (`GameplayStatics.GetObjectClass` _output_get) (`GameplayStatics.GetObjectClass` self)))
    (set `self.HitData` HitData)
    (if (> (`self.Hp`) 0.0)
      (`/Game/Components/StateComponent.SetHittedMode` (`self.StateComponent`))
      (`/Game/Components/WeaponComponent.End_DoAction` (`self.WeaponComponent`))
      (else
        (`/Game/Components/StateComponent.SetDeadMode` (`self.StateComponent`))))))

(event `Hitted`
  (bind (_damage _montage _playratio _canmove _launch _hitstop _sound _shakeclass) (break `/Game/Weapons/FHitData` (`self.HitData`)))
  (bind _attacker (`self.Attacker`)
    (:`then`
      (bind _returnvalue (`self.GetComponentByClass` _attacker "/Game/Components/StateComponent.StateComponent_C"))
      (`/Engine/EditorBlueprintResources/StandardMacros.IsValid` _returnvalue
        (:`Is Valid`
          (bind _output_get (set `self.AttackerSkill` (`/Game/Components/StateComponent.IsSkillMode` _returnvalue)))
          (if _output_get
            (set `self.Damage` (`.Damage_12_F6D23637461C675DE8FC909360F3C064` (break `/Game/Weapons/FHitData` (make `/Game/Weapons/FHitData` 100.0 "/Game/Montages/Damaged/Enemy_Dead_Skill_Montage.Enemy_Dead_Skill_Montage" 1.0 false 100.0 5.0 null "/Game/Weapons/HAmmer/CS_Hammer_Down.CS_Hammer_Down_C" "/Game/TrailPack/Particles/Magic/Hit/P_MagicHitFinisher.P_MagicHitFinisher"))))
            (else
              (set `self.Damage` (`.Damage_12_F6D23637461C675DE8FC909360F3C064` (break `/Game/Weapons/FHitData` (`self.HitData`))))))
          (bind _output_get_2 (set `self.Hp` (`KismetMathLibrary.FClamp` (- (`self.Hp`) (`self.Damage`)) 0.0 (`self.MaxHp`))))
          (if (<= _output_get_2 0.0)
            (set `self.temp` true)
            (`/Game/Components/StateComponent.SetDeadMode` (`self.StateComponent`))
            (`self.PlayAnimMontage` "/Game/Montages/Damaged/Enemy_DeadFall_Montage.Enemy_DeadFall_Montage")
            (`KismetSystemLibrary.Delay` 0.2)
            (`PrimitiveComponent.SetCollisionEnabled` (`self.CapsuleComponent`) "NoCollision")
            (elif (`self.AttackerSkill`)
              (`PlayerCameraManager.StartCameraShake` :`self` (`GameplayStatics.GetPlayerCameraManager` 0) :`ShakeClass` (`.ShakeClass_25_46B57FF54108D96A38CBFF9B8E6FB28B` (break `/Game/Weapons/FHitData` (make `/Game/Weapons/FHitData` 100.0 "/Game/Montages/Damaged/Enemy_Dead_Skill_Montage.Enemy_Dead_Skill_Montage" 1.0 false 100.0 5.0 null "/Game/Weapons/HAmmer/CS_Hammer_Down.CS_Hammer_Down_C" "/Game/TrailPack/Particles/Magic/Hit/P_MagicHitFinisher.P_MagicHitFinisher"))))
              (`self.LaunchCharacter` (* (`self.GetActorForwardVector`) (* (`.Launch_33_ED311C88419A446512768C89386DA5F6` (break `/Game/Weapons/FHitData` (make `/Game/Weapons/FHitData` 100.0 "/Game/Montages/Damaged/Enemy_Dead_Skill_Montage.Enemy_Dead_Skill_Montage" 1.0 false 100.0 5.0 null "/Game/Weapons/HAmmer/CS_Hammer_Down.CS_Hammer_Down_C" "/Game/TrailPack/Particles/Magic/Hit/P_MagicHitFinisher.P_MagicHitFinisher"))) -10.0)))
              (`/Game/Components/StateComponent.SetDownMode` (`self.StateComponent`))
              (if (<= (`self.Hp`) 200.0)
                (bind _asbp_player (cast `/Game/Player/BP_Player` (`self.Attacker`)))
                (`/Game/Components/StateComponent.SetKillMode` (`/Game/Player/BP_Player.StateComponent` _asbp_player))
                (`self.PlayAnimMontage` "/Game/Montages/Paired_1HM_StabStomach_Vic_Montage.Paired_1HM_StabStomach_Vic_Montage")
                (else
                  (`self.PlayAnimMontage` (`.Montage_14_F886CEC54388E9C8406ED7951E41B593` (break `/Game/Weapons/FHitData` (make `/Game/Weapons/FHitData` 100.0 "/Game/Montages/Damaged/Enemy_Dead_Skill_Montage.Enemy_Dead_Skill_Montage" 1.0 false 100.0 5.0 null "/Game/Weapons/HAmmer/CS_Hammer_Down.CS_Hammer_Down_C" "/Game/TrailPack/Particles/Magic/Hit/P_MagicHitFinisher.P_MagicHitFinisher"))))))
              (else
                (`KismetSystemLibrary.PrintString` "none skill" true true (struct :`R` 1.0 :`G` 0.120144 :`A` 1.0))
                (`self.PlayAnimMontage` (`.Montage_14_F886CEC54388E9C8406ED7951E41B593` (break `/Game/Weapons/FHitData` (`self.HitData`))) 2.0)
                (`self.LookAt`)
                (`self.LaunchCharacter` (* (`self.GetActorForwardVector`) (* (`.Launch_33_ED311C88419A446512768C89386DA5F6` (break `/Game/Weapons/FHitData` (`self.HitData`))) -10.0)))
                (if (`KismetSystemLibrary.IsValidClass` _shakeclass)
                  (`PlayerCameraManager.StartCameraShake` :`self` (`GameplayStatics.GetPlayerCameraManager` 0) :`ShakeClass` _shakeclass))))))))
    (:`else`)))

(fn `LimitHeight`
  (bind _maxheight (`self.MaxHeight`))
  (if (>= (.z (`self.K2_GetActorLocation`)) _maxheight)
    (`self.K2_SetActorLocation` (`KismetMathLibrary.MakeVector` (.x (`self.K2_GetActorLocation`)) (.y (`self.K2_GetActorLocation`)) _maxheight))))

(fn `OffParrying`
  (set `self.CanParrying` false))

(fn `OnParrying`
  (set `self.CanParrying` true))

(fn `SetColors`)

(fn `UserConstructionScript`)